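; HomoCommander is a top-down, commander-style camera rig driven by keyboard axes and mouse.
; Collapsed graphs handle axis movement, drag pan or rotate, screen-edge scrolling and zoom, mostly through swept local actor offsets.
; Middle mouse opens gates for dragging and suspends edge scrolling, with a flag choosing pan or rotate (actor yaw, clamped camera pitch).
; The wheel moves the camera along its view axis within height limits measured from InvisibleObject.
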(event `InputAxis|MoveForward`
  (params (AxisValue :type "Float (single-precision)"))
  ;[1 1 1] Camera Directional Movement
  (`self.Camera_MoveForwardAndRight` AxisValue (stale `InputAxis|MoveRight` AxisValue) :!label _label))

(event `InputAxis|MoveRight`
  (params (AxisValue :type "Float (single-precision)"))
  ;[1 1 1] Camera Directional Movement
  (goto _label :!via `LeftAndRight`))

(event `Key|MouseScrollUp`
  (params (Key :type "Key Structure" :default "AnyKey"))
  ;[1 1 1] Camera Zoom
  (:`Pressed`
    (`self.Camera_Zoom` :!label _label_2)))

(event `Key|MouseScrollDown`
  (params (Key :type "Key Structure" :default "AnyKey"))
  ;[1 1 1] Camera Zoom
  (:`Pressed`
    (goto _label_2 :!via `ZoomOut`)))

(event `InputAxisKey|MouseX`
  (params (AxisValue :type "Float (single-precision)"))
  ;[1 1 1] Camera Pan/Rotate
  (`/Engine/EditorBlueprintResources/StandardMacros.Gate` true :!label _label_3
    (:`Exit`
      (if (`self.Camera_TPanFRotate`)
        (`self.Camera_Pan` AxisValue (stale `InputAxisKey|MouseY` AxisValue) :!label _label_4)
        (else
          (`self.Camera_Rotate` AxisValue (stale `InputAxisKey|MouseY` AxisValue) :!label _label_5))))))

(event `Key|MiddleMouseButton`
  (params (Key :type "Key Structure" :default "AnyKey"))
  ;[1 1 1] Camera Pan/Rotate
  (:`Pressed`
    (set `self.Camera_ScreenEdgeHitEnabled` false)
    (`|ExecutionSequence`
      (:`then_0`
        (goto _label_3 :!via `Open`))
      (:`then_1`
        (goto _label_6 :!via `Open`))))
  (:`Released`
    (set `self.Camera_ScreenEdgeHitEnabled` true)
    (`|ExecutionSequence`
      (:`then_0`
        (goto _label_3 :!via `Close`))
      (:`then_1`
        (goto _label_6 :!via `Close`)))))

(event `InputAxisKey|MouseY`
  (params (AxisValue :type "Float (single-precision)"))
  ;[1 1 1] Camera Pan/Rotate
  (`/Engine/EditorBlueprintResources/StandardMacros.Gate` true :!label _label_6
    (:`Exit`
      (if (`self.Camera_TPanFRotate`)
        (goto _label_4 :!via `MouseY`)
        (else
          (goto _label_5 :!via `MouseY`))))))

(event `InputAxisKey|MouseX`
  (params (AxisValue :type "Float (single-precision)"))
  ;[1 1 1] Camera Screen Edge Hit
  (if (`self.Camera_ScreenEdgeHitEnabled`)
    (`self.Camera_ScreenEdgeHit` :!label _label_7)))

(event `InputAxisKey|MouseY`
  (params (AxisValue :type "Float (single-precision)"))
  ;[1 1 1] Camera Screen Edge Hit
  (if (`self.Camera_ScreenEdgeHitEnabled`)
    (goto _label_7 :!via `ForwardAndBack`)))

(fn `UserConstructionScript`)