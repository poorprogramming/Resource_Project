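; Grid actor that builds the tile map at BeginPlay from the Map array stored in Resource_Game_Instance.
; It spawns an indexed Empty_Tile for every cell, deriving positions from the grid dimensions and tile size.
; Tiles alternate Clear_Black and Clear_White materials in a checkerboard whose row parity assumes 10 cells per row.
; Cells marked Cave or Path also get a visible 00Cave or Path_Blueprint actor at the same transform.
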(event `self.ReceiveBeginPlay`
  (bind _small_tile_size (`self.Small_Tile_Size`))
  (bind _spawn_transform (`self.Spawn_Transform`))
  (bind _y_hight (`self.Y_Hight`))
  (bind _index (`self.index`))
  (bind _asresource_game_instance (cast `/Game/Resource_Game_Instance` (`GameplayStatics.GetGameInstance`)))
  (set `self.Game Instance` _asresource_game_instance)
  (for _index_2 (range (* (`self.X_Width`) (`self.Y_Hight`)))
    (bind _output_get (set `self.index` _index_2))
    (bind _output_get_2 (set `self.Spawn_Transform` (`KismetMathLibrary.Conv_VectorToTransform` (`KismetMathLibrary.MakeVector` (`KismetMathLibrary.Conv_IntToDouble` (* (/ _output_get _y_hight) _small_tile_size)) (`KismetMathLibrary.Conv_IntToDouble` (* (mod _output_get _y_hight) _small_tile_size))))))
    (bind _returnvalue (`|SpawnActorFromClass` "/Game/Blueprints/Empty_Tile.Empty_Tile_C" _output_get_2 "AlwaysSpawn" "OverrideRootScale"))
    (set `/Game/Blueprints/Empty_Tile.Map_Index` (`self.index`) _returnvalue)
    (`PrimitiveComponent.SetMaterial` (`StaticMeshActor.StaticMeshComponent` _returnvalue) 0 (select `bool` (xor (`KismetMathLibrary.Conv_IntToBool` (mod _index 2)) (`KismetMathLibrary.Conv_IntToBool` (mod (/ _index 10) 2))) :`false` "/Game/Materials/Tile/Clear_White.Clear_White" :`true` "/Game/Materials/Tile/Clear_Black.Clear_Black" :!type "Material Object Reference"))
    (switch `string` (`KismetArrayLibrary.Array_Get` (`/Game/Resource_Game_Instance.Map` (`self.Game Instance`)) (`self.index`))
      (:`Cave`
        (bind _returnvalue_2 (`|SpawnActorFromClass` "/Game/Blueprints/Source/00Cave.00Cave_C" _spawn_transform "Undefined" "OverrideRootScale"))
        (`self.SetActorHiddenInGame` _returnvalue_2 false))
      (:`Path`
        (bind _returnvalue_3 (`|SpawnActorFromClass` "/Game/Blueprints/Path_Blueprint.Path_Blueprint_C" _spawn_transform "Undefined" "OverrideRootScale"))
        (`self.SetActorHiddenInGame` _returnvalue_3 false)))))

(fn `UserConstructionScript`)