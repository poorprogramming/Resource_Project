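; Path_Generate is a grid-path actor that builds a tile border in its construction script, with no active runtime logic.
; PopulateBorderArray fills an array with flat edge indices, though two loops end at a hardcoded offset from Size and one repeats a single corner index.
; When DisplayBorder is set, SpawnInstances maps each index through TileToGrid, scales it by TileSize and adds an instance to the Path mesh.
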(event `self.ReceiveBeginPlay`)

(event `self.ReceiveActorBeginOverlap`
  (params (OtherActor :type "Actor Object Reference")))

(event `self.ReceiveTick`
  (params (DeltaSeconds :type "Float (single-precision)")))

(fn `Populate_Border_Array`
  (params (Size :type Integer) (Border_Array :type "Array of Integer"))
  (bind _x_size (`self.X_Size`))
  (set `self.X_Size` Size)
  (for _index (range _x_size)
    (`KismetArrayLibrary.Array_Add` Border_Array _index))
  (for _index_2 (range (+ (- _x_size 52) 1))
    (`KismetArrayLibrary.Array_Add` Border_Array (+ (* _index_2 0) (- _x_size 1))))
  (for _index_3 (range (+ _x_size 1))
    (`KismetArrayLibrary.Array_Add` Border_Array (+ (- _index_3 1) (* _x_size (- _x_size 1)))))
  (for _index_4 (range (+ (- (`self.X_Size`) 52) 1))
    (`KismetArrayLibrary.Array_Add` Border_Array (* _index_4 _x_size))))

(fn `UserConstructionScript`
  (`self.Populate_Border_Array` (`self.Size`) (`self.Border_Tiles`))
  (if (`self.Display_Border`)
    (`self.Spawn_Instances` (`self.Border_Tiles`) (`self.Size`) (`self.Tile_Size`) (1.0 1.0 1.0) (`self.Path`))))