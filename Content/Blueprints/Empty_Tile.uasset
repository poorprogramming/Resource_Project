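; Empty_Tile is a clickable empty map tile where the player places the element currently being spawned, either a Cave or a Path.
; Hovering highlights it through a dynamic material, plays a randomly picked sound and moves the element's preview actor onto valid tiles.
; FMapCheck validates by index math on a ten-wide grid: Caves need interior tiles, Paths need tiles orthogonally adjacent to the Cave.
; A valid click writes the Game Instance map and unlocks follow-on elements.
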(event MouseInput|EventActorEndCursorOver
  ;[1 1 1] EndCursorOver
  (bind _isvalid (CallFunction|FMapCheck))
  (if _isvalid
    (Rendering|SetActorHiddenInGame (.Actor (Utilities|Struct|BreakSpawn_Element (Variables|/Game/Resource_Game_Instance.Resource_Game_Instance_C|GetSpawn%20Element (Variables|Default|GetGame%20Instance)))) true))
  (Rendering|Material|SetVectorParameterValue :self (Variables|Default|GetDynamic_Material) :ParameterName "clear" :!class /Script/Engine.MaterialInstanceDynamic))

(event MouseInput|EventActorOnClicked
  (bind _game_instance (Variables|Default|GetGame%20Instance))
  (bind _game_instance_2 (Variables|Default|GetGame%20Instance))
  (bind _game_instance_3 (Variables|Default|GetGame%20Instance))
  ;[1 1 1] OnClicked
  (Math|Integer|IncrementInt (Variables|/Game/Resource_Game_Instance.Resource_Game_Instance_C|GetClicks (Variables|Default|GetGame%20Instance))
    (:%20%20
      (bind _isvalid (CallFunction|FMapCheck))
      (if _isvalid
        (switch int (.Element_Code (Utilities|Struct|BreakSpawn_Element (Variables|/Game/Resource_Game_Instance.Resource_Game_Instance_C|GetSpawn%20Element (Variables|Default|GetGame%20Instance))))
          (:1
            ;[1 1 1] Cave
            (Utilities|Array|SetArrayElem (Variables|/Game/Resource_Game_Instance.Resource_Game_Instance_C|GetMap (Variables|Default|GetGame%20Instance)) (Variables|Default|GetMap_Index) 1)
            (Variables|/Game/Resource_Game_Instance.Resource_Game_Instance_C|SetSpawn%20Element _game_instance_2 "")
            (Utilities|Struct|SetmembersinElement (Variables|/Game/Resource_Game_Instance.Resource_Game_Instance_C|GetHomo _game_instance_2) false)
            (Utilities|Struct|SetmembersinElement (Variables|/Game/Resource_Game_Instance.Resource_Game_Instance_C|GetAir _game_instance_2) false true)
            (Utilities|Struct|SetmembersinElement (Variables|/Game/Resource_Game_Instance.Resource_Game_Instance_C|GetPath _game_instance_2) false))
          (:2
            ;[1 1 1] Path
            (Utilities|Array|SetArrayElem (Variables|/Game/Resource_Game_Instance.Resource_Game_Instance_C|GetMap _game_instance_3) (Variables|Default|GetMap_Index) 2)
            (Variables|/Game/Resource_Game_Instance.Resource_Game_Instance_C|SetSpawn%20Element _game_instance_3 "")
            (Math|Integer|IncrementInt (.active (Variables|/Game/Resource_Game_Instance.Resource_Game_Instance_C|GetPath _game_instance_3))
              (:%20%20
                (Utilities|Struct|SetmembersinElement (Variables|/Game/Resource_Game_Instance.Resource_Game_Instance_C|GetWater_Body _game_instance) false)
                (Utilities|Struct|SetmembersinElement (Variables|/Game/Resource_Game_Instance.Resource_Game_Instance_C|GetPlains _game_instance) false)))))
        (Rendering|Material|SetVectorParameterValue :self (Variables|Default|GetDynamic_Material) :ParameterName "clear" :!class /Script/Engine.MaterialInstanceDynamic)
        (AddComponent|AddAudioComponent false)))))

(event EventBeginPlay
  ;[1 1 1] BeginPlay
  (bind _asresource_game_instance (Utilities|Casting|CastToResource_Game_Instance (Game|GetGameInstance)))
  (Variables|Default|SetGame%20Instance _asresource_game_instance))

(event MouseInput|EventActorBeginCursorOver
  (bind _game_instance (Variables|Default|GetGame%20Instance))
  (bind _spawn_element (Variables|/Game/Resource_Game_Instance.Resource_Game_Instance_C|GetSpawn%20Element _game_instance))
  (bind _actor (Utilities|Struct|BreakSpawn_Element _spawn_element))
  ;[1 1 1] BeginCursorOver
  (bind _isvalid (CallFunction|FMapCheck))
  (if _isvalid
    (Rendering|SetActorHiddenInGame _actor false)
    (Transformation|SetActorLocation _actor (Transformation|GetActorLocation) false false))
  (Rendering|Material|SetVectorParameterValue (Variables|Default|GetDynamic_Material) "Clear" "(R=1.000000,G=1.000000,B=1.000000,A=1.000000)" :!class /Script/Engine.MaterialInstanceDynamic)
  ;[1 1 1] Sound
  (Utilities|FlowControl|MultiGate true false -1
    (:Out%200
      (AddComponent|AddAudioComponent false))
    (:Out%201
      (AddComponent|AddAudioComponent false))
    (:Out%202
      (AddComponent|AddAudioComponent false))
    (:Out%203
      (AddComponent|AddAudioComponent false))
    (:Out%204
      (AddComponent|AddAudioComponent false))
    (:Out%205
      (AddComponent|AddAudioComponent false))))

(fn ConstructionScript
  (bind _returnvalue (Rendering|Material|CreateDynamicMaterialInstance (Variables|Debug|GetStaticMeshComponent) 0 0 :!class /Script/Engine.PrimitiveComponent))
  (Variables|Default|SetDynamic_Material _returnvalue))

(fn FMapCheck
  (bind _game_instance (Variables|Default|GetGame%20Instance))
  (bind _spawn_element (Variables|/Game/Resource_Game_Instance.Resource_Game_Instance_C|GetSpawn%20Element _game_instance))
  (bind (_spawning _actor _element_code) (Utilities|Struct|BreakSpawn_Element _spawn_element))
  (if _spawning
    (switch int _element_code
      (:Default
        _)
      (:0
        _)
      (:1
        ;[1 1 1] Cave
        (if (|((((MapIndex>10)&&(MapIndex<90))&&((MapIndex%10)!=0))&&(((MapIndex+1)%10)!=0)) (Variables|Default|GetMap_Index))
          (return true)
          (else
            (return false))))
      (:2
        ;[1 1 1] Path
        (if (|(((((CaveIndex-1)==MapIndex)||((CaveIndex+1)==MapIndex))||((CaveIndex-10)==MapIndex))||((CaveIndex+10)==MapIndex)) (Utilities|Array|FindItem (Variables|/Game/Resource_Game_Instance.Resource_Game_Instance_C|GetMap (Variables|Default|GetGame%20Instance)) 1) (Variables|Default|GetMap_Index))
          (return true)
          (else
            (return false))))))
  (return false))