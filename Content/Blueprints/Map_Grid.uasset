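; Map_Grid is an actor that lays out a tile grid sized by XWidth, YHight and SmallTileSize.
; Its construction script adds a static mesh component per cell at actor-relative offsets, deriving column and row from one loop index by division and modulo.
; When the cursor moves over it, it spawns a Grid actor per cell using those offsets as world positions, with no guard against repeat spawning.
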(event `self.ReceiveActorBeginCursorOver`
  (bind _small_tile_size (`self.Small_Tile_Size`))
  (bind _y_hight (`self.Y_Hight`))
  (for _index (range (* (`self.X_Width`) (`self.Y_Hight`)))
    (`|SpawnActorFromClass` "/Game/Blueprints/Grid.Grid_C" (`KismetMathLibrary.Conv_VectorToTransform` (`KismetMathLibrary.MakeVector` (`KismetMathLibrary.Conv_IntToDouble` (* (/ _index _y_hight) _small_tile_size)) (`KismetMathLibrary.Conv_IntToDouble` (* (mod _index _y_hight) _small_tile_size)))) true)))

(event `self.ReceiveTick`
  (params (DeltaSeconds :type "Float (single-precision)")))

(fn `UserConstructionScript`
  (bind _small_tile_size (`self.Small_Tile_Size`))
  (bind _y_hight (`self.Y_Hight`))
  (for _index (range (* (`self.X_Width`) (`self.Y_Hight`)))
    (`AddComponent|Static Mesh Component_13188` :`RelativeTransform` (`KismetMathLibrary.Conv_VectorToTransform` (`KismetMathLibrary.MakeVector` (`KismetMathLibrary.Conv_IntToDouble` (* (/ _index _y_hight) _small_tile_size)) (`KismetMathLibrary.Conv_IntToDouble` (* (mod _index _y_hight) _small_tile_size)))))))