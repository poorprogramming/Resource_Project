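; Map grid spawner actor that builds the tile map at BeginPlay from the Map array in Resource_Game_Instance.
; It spawns an Empty_Tile per cell, registers it in TileMap, and sets its index, row, column and checkerboard material, with the checker pattern assuming 10 cells per line.
; SpawnElement then spawns the matching terrain or structure actor there, adds it to ActorMap and stores that index on the tile.
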(event EventBeginPlay
  (bind _small_tile_size (Variables|Default|GetSmall_Tile_Size))
  (bind _y_hight (Variables|Default|GetY_Hight))
  (bind _asresource_game_instance (Utilities|Casting|CastToResource_Game_Instance (Game|GetGameInstance)))
  (Variables|Default|SetGame%20Instance _asresource_game_instance)
  (for _index (range 0 (- (* (Variables|Default|GetX_Width) (Variables|Default|GetY_Hight)) 1))
    (bind _output_get (Variables|Default|Setindex _index))
    (bind _output_get_2 (Variables|Default|SetSpawn_Transform (Math|Conversions|ToTransform(Vector) (Math|Vector|MakeVector (Math|Conversions|ToFloat(Integer) (* (/ _output_get _y_hight) _small_tile_size)) (Math|Conversions|ToFloat(Integer) (* (Math|Integer|%(Integer) _output_get _y_hight) _small_tile_size)) -9.9))))
    (bind _returnvalue (Game|SpawnActorfromClass "/Game/Blueprints/MiscActors/Empty_Tile.Empty_Tile_C" _output_get_2 "AlwaysSpawn" 0 0))
    (bind _output_get_3 (Variables|Default|SetEmpty%20Tile _returnvalue))
    (bind _returnvalue_2 (Utilities|Array|AddUnique (Variables|/Game/Resource_Game_Instance.Resource_Game_Instance_C|GetTile%20Map (Variables|Default|GetGame%20Instance)) _output_get_3))
    (Variables|/Game/Blueprints/MiscActors/Empty_Tile.Empty_Tile_C|Setindex (Variables|Default|GetEmpty%20Tile) _returnvalue_2)
    (Variables|/Game/Blueprints/MiscActors/Empty_Tile.Empty_Tile_C|SetRow (Variables|Default|GetEmpty%20Tile) (|(floor(({EF5DE6BE-4506-93B2-743F-F496D309CCFD}/10)))))
    (Variables|/Game/Blueprints/MiscActors/Empty_Tile.Empty_Tile_C|SetColumn (Variables|Default|GetEmpty%20Tile) (|({EF5DE6BE-4506-93B2-743F-F496D309CCFD}%10)))
    (Variables|/Game/Blueprints/MiscActors/Empty_Tile.Empty_Tile_C|SetMaterial (Variables|Default|GetEmpty%20Tile) (select (Class|KismetMathLibrary|XORBoolean (Math|Conversions|ToBoolean(Integer) (Math|Integer|%(Integer) (Variables|Default|Getindex) 2)) (Math|Conversions|ToBoolean(Integer) (Math|Integer|%(Integer) (/ (Variables|Default|Getindex) 10) 2))) "/Game/Materials/Tile_Materials/Black.Black" "/Game/Materials/Tile_Materials/White.White"))
    (switch string (Utilities|Array|Get(acopy) (Variables|/Game/Resource_Game_Instance.Resource_Game_Instance_C|GetMap (Variables|Default|GetGame%20Instance)) (Variables|Default|Getindex))
      (:Cave
        (CallFunction|SpawnElement "/Game/Blueprints/Source/00Cave.00Cave_C"))
      (:Path
        (CallFunction|SpawnElement "/Game/Blueprints/MiscActors/XXPath_Blueprint.XXPath_Blueprint_C"))
      (:Water%20Body
        (CallFunction|SpawnElement "/Game/Blueprints/Source/01Water_Body.01Water_Body_C"))
      (:Plains
        (CallFunction|SpawnElement "/Game/Blueprints/Source/02Plains.02Plains_C"))
      (:Forest
        (CallFunction|SpawnElement "/Game/Blueprints/Source/03Forest.03Forest_C"))
      (:Mountain
        (CallFunction|SpawnElement "/Game/Blueprints/Source/04Mountain.04Mountain_C"))
      (:Hut
        (CallFunction|SpawnElement "/Game/Blueprints/Source/05Hut.05Hut_C"))
      (:Fire%20Pit
        (CallFunction|SpawnElement "/Game/Blueprints/Source/06Fire_Pit.06Fire_Pit_C"))
      (:Altar
        (CallFunction|SpawnElement "/Game/Blueprints/Source/07Altar.07Altar_C")))))

(fn ConstructionScript)

(fn SpawnElement
  (params (Class :type Actor%20Class%20Reference))
  (bind _returnvalue (Game|SpawnActorfromClass Class (Variables|Default|GetSpawn_Transform) "Undefined" 0 0))
  (Rendering|SetActorHiddenInGame _returnvalue false)
  (bind _returnvalue_2 (Utilities|Array|Add (Variables|/Game/Resource_Game_Instance.Resource_Game_Instance_C|GetActor%20Map (Variables|Default|GetGame%20Instance)) _returnvalue))
  (Variables|/Game/Blueprints/MiscActors/Empty_Tile.Empty_Tile_C|Setactor%20index (Variables|Default|GetEmpty%20Tile) _returnvalue_2)
  (return))