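; BigNumber is an actor that stores very large values as a float mantissa and integer exponent, with arithmetic, comparison and display functions.
; NormalizeMantissa keeps values in scientific form, while add and subtract temporarily align their inputs' exponents, with subtraction clamping negative mantissas to zero.
; Operations write into a caller-supplied destination, and powers use repeated multiplication with temporary spawned BigNumber actors.
; ToString shows postfixes from BigNumPostfix, falling back to exponential notation beyond them.
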(fn ConstructionScript)

(fn GetBigNumberMantissa
  (return (Variables|Default|GetMantissa)))

(fn GetBigNumberExponent
  (return (Variables|Default|GetExponent)))

(fn MakeNewBigNumber
  (params (inFloat :type Float%20%28single-precision%29) (inExponent :type Integer))
  (Variables|Default|SetMantissa inFloat)
  (Variables|Default|SetExponent inExponent)
  (Internal|NormalizeMantissa)
  (return self))

(fn NormalizeMantissa
  (if (== (Variables|Default|GetMantissa) 0.0)
    ;[1 1 1] Mantissa was 0.  Set Exponent to 0 too.
    (Variables|Default|SetExponent 0)
    (else
      ;[1 1 1] If the Mantissa is less than 1, get it up there and decrement the Exponent
      (while (< (Variables|Default|GetMantissa) 1.0)
        (Variables|Default|SetMantissa (* (Variables|Default|GetMantissa) 1e+01))
        (Variables|Default|SetExponent (- (Variables|Default|GetExponent) 1)))
      ;[1 1 1] If the Mantissa is >= 10, bring it down and increment the Exponent
      (while (>= (Variables|Default|GetMantissa) 1e+01)
        (Variables|Default|SetMantissa (/ (Variables|Default|GetMantissa) 1e+01))
        (Variables|Default|SetExponent (+ (Variables|Default|GetExponent) 1))))))

(fn SetBigNumberMantissa
  (params (NewParam :type Float%20%28single-precision%29))
  (Variables|Default|SetMantissa NewParam))

(fn SetBigNumberExponent
  (params (Exponent :type Integer))
  (Variables|Default|SetExponent Exponent))

(fn RaisetoLargestExponent
  (params (InBigNumber1 :type Big%20Number%20Object%20Reference) (InBigNumber2 :type Big%20Number%20Object%20Reference))
  (bind _exponent (VariableAccess|GetBigNumberExponent InBigNumber1))
  (bind _exponent_2 (VariableAccess|GetBigNumberExponent InBigNumber2))
  ;[1 1 1] Make sure these numbers are valid
  (if (and (Utilities|IsValid InBigNumber1) (Utilities|IsValid InBigNumber2))
    (if (or (== (Variables|BigNumber_C|GetMantissa InBigNumber1) 0.0) (== (Variables|BigNumber_C|GetMantissa InBigNumber2) 0.0))
      _
      (else
        (while (< _exponent _exponent_2)
          (VariableAccess|SetBigNumberMantissa InBigNumber1 (/ (VariableAccess|GetBigNumberMantissa InBigNumber1) 1e+01))
          (VariableAccess|SetBigNumberExponent InBigNumber1 (+ _exponent 1)))
        (while (< _exponent_2 _exponent)
          (VariableAccess|SetBigNumberMantissa InBigNumber2 (/ (VariableAccess|GetBigNumberMantissa InBigNumber2) 1e+01))
          (VariableAccess|SetBigNumberExponent InBigNumber2 (+ _exponent_2 1))))))
  (return InBigNumber1 InBigNumber2))

(fn ToStringExp
  (return (Utilities|String|BuildString(Integer) (Utilities|String|GetSubstring (Utilities|String|BuildString(Float) "" "" (Variables|Default|GetMantissa)) 0 6) "E" (Variables|Default|GetExponent))))

(fn AddBigNumbers
  (params (InBigNum1 :type Big%20Number%20Object%20Reference) (InBigNum2 :type Big%20Number%20Object%20Reference) (DestBigNumber :type Big%20Number%20Object%20Reference))
  (bind (_outbignumber1 _outbignumber2) (Internal|RaisetoLargestExponent InBigNum1 InBigNum2))
  (VariableAccess|SetBigNumberMantissa DestBigNumber (+ (VariableAccess|GetBigNumberMantissa _outbignumber1) (VariableAccess|GetBigNumberMantissa _outbignumber2)))
  (Internal|NormalizeMantissa DestBigNumber)
  (Internal|NormalizeMantissa InBigNum1)
  (Internal|NormalizeMantissa InBigNum2)
  (return DestBigNumber))

(fn SubtractBigNumbers
  (params (InBigNum1 :type Big%20Number%20Object%20Reference) (InBigNum2 :type Big%20Number%20Object%20Reference) (DestBigNumber :type Big%20Number%20Object%20Reference))
  (bind (_outbignumber1 _outbignumber2) (Internal|RaisetoLargestExponent InBigNum1 InBigNum2))
  (VariableAccess|SetBigNumberMantissa DestBigNumber (Math|Float|Max(Float) (- (VariableAccess|GetBigNumberMantissa _outbignumber1) (VariableAccess|GetBigNumberMantissa _outbignumber2)) 0.0))
  (Internal|NormalizeMantissa DestBigNumber)
  (Internal|NormalizeMantissa InBigNum1)
  (Internal|NormalizeMantissa InBigNum2)
  (return DestBigNumber))

(fn MultiplyBigNumbers
  (params (InBigNum1 :type Big%20Number%20Object%20Reference) (InBigNum2 :type Big%20Number%20Object%20Reference) (DestBigNumber :type Big%20Number%20Object%20Reference))
  (VariableAccess|SetBigNumberMantissa DestBigNumber (* (VariableAccess|GetBigNumberMantissa InBigNum1) (VariableAccess|GetBigNumberMantissa InBigNum2)))
  (VariableAccess|SetBigNumberExponent DestBigNumber (+ (VariableAccess|GetBigNumberExponent InBigNum1) (VariableAccess|GetBigNumberExponent InBigNum2)))
  (Internal|NormalizeMantissa DestBigNumber)
  (return DestBigNumber))

(fn MultiplyBigNumberbyFloat
  (params (InBigNum1 :type Big%20Number%20Object%20Reference) (InFloat :type Float%20%28single-precision%29) (DestBigNumber :type Big%20Number%20Object%20Reference))
  (VariableAccess|SetBigNumberMantissa DestBigNumber (* (VariableAccess|GetBigNumberMantissa InBigNum1) InFloat))
  (VariableAccess|SetBigNumberExponent DestBigNumber (VariableAccess|GetBigNumberExponent InBigNum1))
  (Internal|NormalizeMantissa DestBigNumber)
  (return DestBigNumber))

(fn DivideBigNumberbyFloat
  (params (InBigNum1 :type Big%20Number%20Object%20Reference) (InFloat :type Float%20%28single-precision%29) (DestBigNumber :type Big%20Number%20Object%20Reference))
  (VariableAccess|SetBigNumberMantissa DestBigNumber (/ (VariableAccess|GetBigNumberMantissa InBigNum1) InFloat))
  (VariableAccess|SetBigNumberExponent DestBigNumber (VariableAccess|GetBigNumberExponent))
  (Internal|NormalizeMantissa DestBigNumber)
  (return DestBigNumber))

(fn LowertoSmallestExponent
  (params (InBigNumber1 :type Big%20Number%20Object%20Reference) (InBigNumber2 :type Big%20Number%20Object%20Reference))
  (bind _exponent (VariableAccess|GetBigNumberExponent InBigNumber1))
  (bind _exponent_2 (VariableAccess|GetBigNumberExponent InBigNumber2))
  (while (> _exponent _exponent_2)
    (VariableAccess|SetBigNumberMantissa InBigNumber1 (* (VariableAccess|GetBigNumberMantissa InBigNumber1) 1e+01))
    (VariableAccess|SetBigNumberExponent InBigNumber1 (- _exponent 1)))
  (while (> _exponent_2 _exponent)
    (VariableAccess|SetBigNumberMantissa InBigNumber2 (* (VariableAccess|GetBigNumberMantissa InBigNumber2) 1e+01))
    (VariableAccess|SetBigNumberExponent InBigNumber2 (- _exponent_2 1)))
  (return InBigNumber1 InBigNumber2))

(fn DivideBigNumbers
  (params (InBigNum1 :type Big%20Number%20Object%20Reference) (InBigNum2 :type Big%20Number%20Object%20Reference) (DestBigNumber :type Big%20Number%20Object%20Reference))
  (VariableAccess|SetBigNumberMantissa DestBigNumber (/ (VariableAccess|GetBigNumberMantissa InBigNum1) (VariableAccess|GetBigNumberMantissa InBigNum2)))
  (VariableAccess|SetBigNumberExponent DestBigNumber (- (VariableAccess|GetBigNumberExponent InBigNum1) (VariableAccess|GetBigNumberExponent InBigNum2)))
  (Internal|NormalizeMantissa DestBigNumber)
  (return DestBigNumber))

(fn ToString
  (bind _exponent (Variables|Default|GetExponent))
  (bind _mantissa (Variables|Default|GetMantissa))
  (bind _returnvalue (Math|Conversions|ToFloat(Integer) _exponent))
  (bind _returnvalue_2 (|(x*(pow(10,y))) _mantissa _returnvalue))
  (if (< (Variables|Default|GetExponent) 3)
    ;[1 1 1] Number less than 1000, just show it.
    (if (Math|Float|InRange(Float) _returnvalue_2 0.0 1.0 false false)
      (return "1")
      (else
        (return (Utilities|String|ToString(Integer) (Math|Float|Floor _returnvalue_2)))))
    (elif (> (/ (Variables|Default|GetExponent) 3) 201)
      (bind _outstring (OutputStrings|ToStringExp))
      (return _outstring)
      (else
        (return (Utilities|String|Append (Utilities|String|GetSubstring (Utilities|String|BuildString(Float) "" "" (|(x*(pow(10,y))) (Variables|Default|GetMantissa) (Math|Conversions|ToFloat(Integer) (Math|Integer|%(Integer) (Variables|Default|GetExponent) 3)))) 0 5) (Utilities|Array|Get(acopy) (Variables|Default|GetBigNumPostfix) (/ (Variables|Default|GetExponent) 3))))))))

(fn BigNumberLessThan
  (params (BigNumber1 :type Big%20Number%20Object%20Reference) (BigNumber2 :type Big%20Number%20Object%20Reference))
  (bind _exponent (VariableAccess|GetBigNumberExponent BigNumber1))
  (bind _exponent_2 (VariableAccess|GetBigNumberExponent BigNumber2))
  (if (and (Utilities|IsValid BigNumber2) (Utilities|IsValid BigNumber1))
    (if (< _exponent _exponent_2)
      (return true)
      (elif (> _exponent _exponent_2)
        (return false)
        (elif (< (VariableAccess|GetBigNumberMantissa BigNumber1) (VariableAccess|GetBigNumberMantissa BigNumber2))
          (return true)
          (else
            (return false)))))
    (else
      (return true))))

(fn BigNumberGreaterThan
  (params (BigNumber1 :type Big%20Number%20Object%20Reference) (BigNumber2 :type Big%20Number%20Object%20Reference))
  (bind _exponent (VariableAccess|GetBigNumberExponent BigNumber1))
  (bind _exponent_2 (VariableAccess|GetBigNumberExponent BigNumber2))
  (if (> _exponent _exponent_2)
    (return true)
    (elif (< _exponent _exponent_2)
      (return false)
      (elif (> (VariableAccess|GetBigNumberMantissa BigNumber1) (VariableAccess|GetBigNumberMantissa BigNumber2))
        (return true)
        (else
          (return false))))))

(fn BigNumberEqualto
  (params (BigNumber1 :type Big%20Number%20Object%20Reference) (BigNumber2 :type Big%20Number%20Object%20Reference))
  (return (and (== (VariableAccess|GetBigNumberExponent BigNumber1) (VariableAccess|GetBigNumberExponent BigNumber2)) (== (VariableAccess|GetBigNumberMantissa BigNumber1) (VariableAccess|GetBigNumberMantissa BigNumber2)))))

(fn BigNumberPower
  (params (BigNumberIn :type Big%20Number%20Object%20Reference) (BigNumberPower :type Integer) (BigNumberDest :type Big%20Number%20Object%20Reference))
  (bind _mantissa (VariableAccess|GetBigNumberMantissa BigNumberIn))
  (bind _exponent (VariableAccess|GetBigNumberExponent BigNumberIn))
  (bind _returnvalue (Game|SpawnActorfromClass "BigNumber_C" (Transformation|GetActorTransform) "Undefined" 0 _mantissa _exponent))
  (bind _output_get (Variables|Default|SetTempBigNum _returnvalue))
  (VariableAccess|SetBigNumberMantissa BigNumberDest _mantissa)
  (VariableAccess|SetBigNumberExponent BigNumberDest _exponent)
  (while (> BigNumberPower 1)
    (Maths|MultiplyBigNumbers BigNumberDest BigNumberDest _output_get BigNumberDest)
    (Math|Integer|DecrementInt BigNumberPower))
  (Actor|DestroyActor _output_get)
  (return BigNumberDest))

(fn DivideBigNumbersReturnFloat
  (params (InBigNum1 :type Big%20Number%20Object%20Reference) (InBigNum2 :type Big%20Number%20Object%20Reference))
  (return (|(x*(pow(10,y))) (/ (VariableAccess|GetBigNumberMantissa InBigNum1) (VariableAccess|GetBigNumberMantissa InBigNum2)) (Math|Conversions|ToFloat(Integer) (- (VariableAccess|GetBigNumberExponent InBigNum1) (VariableAccess|GetBigNumberExponent InBigNum2))))))

(fn BigNumbersPower
  (params (BigNumberIn :type Big%20Number%20Object%20Reference) (BigNumberPower :type Big%20Number%20Object%20Reference) (BigNumberDest :type Big%20Number%20Object%20Reference))
  (bind _mantissa (VariableAccess|GetBigNumberMantissa BigNumberIn))
  (bind _exponent (VariableAccess|GetBigNumberExponent BigNumberIn))
  (bind _returnvalue (Game|SpawnActorfromClass "BigNumber_C" (Transformation|GetActorTransform) "Undefined" 0 _mantissa _exponent))
  (bind _output_get (Variables|Default|SetTempBigNum _returnvalue))
  (VariableAccess|SetBigNumberMantissa BigNumberDest _mantissa)
  (VariableAccess|SetBigNumberExponent BigNumberDest _exponent)
  (while (Maths|BigNumberGreaterThanOne BigNumberPower)
    (Maths|MultiplyBigNumbers BigNumberDest BigNumberDest _output_get BigNumberDest)
    ;[1 1 1] decrement 1
    (bind _returnvalue_2 (Game|SpawnActorfromClass "BigNumber_C" (Transformation|GetActorTransform) "Undefined" 0 1.0 0))
    (Maths|SubtractBigNumbers BigNumberPower BigNumberPower _returnvalue_2 BigNumberPower)
    (Actor|DestroyActor _returnvalue_2))
  (Actor|DestroyActor _output_get)
  (return BigNumberDest))

(fn BigNumberGreaterThanOne
  (params (BigNumber1 :type Big%20Number%20Object%20Reference))
  (bind _exponent (VariableAccess|GetBigNumberExponent BigNumber1))
  (if (> _exponent 1)
    (return true)
    (elif (< _exponent 1)
      (return false)
      (elif (> (VariableAccess|GetBigNumberMantissa BigNumber1) 1.0)
        (return true)
        (else
          (return false))))))