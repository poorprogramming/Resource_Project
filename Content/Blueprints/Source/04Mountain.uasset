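; 04Mountain is the Mountain resource source, which advances the resource elements tied to the mountain over time.
; On BeginPlay it caches the Resource_Game_Instance.
; Every Tick it passes delta time to that instance's Progress function for Hammerstone, Flint, GroundStone and EvilSpirit, with Mountain as the Source.
; The element data and progress logic live in the game instance, so this Blueprint only drives the updates.
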(event `self.ReceiveBeginPlay`
  ;[1 1 1] BeginPlay
  (bind _asresource_game_instance (cast `/Game/Resource_Game_Instance` (`GameplayStatics.GetGameInstance`)))
  (set `self.Game Instance` _asresource_game_instance))

(event `self.ReceiveTick`
  (params (DeltaSeconds :type "Float (single-precision)"))
  (bind _game_instance (`self.Game Instance`))
  (bind _mountain (`/Game/Resource_Game_Instance.Mountain` _game_instance))
  (`/Game/Resource_Game_Instance.Progress++` _game_instance DeltaSeconds (`/Game/Resource_Game_Instance.Hammerstone` _game_instance) _mountain false)
  (`/Game/Resource_Game_Instance.Progress++` _game_instance DeltaSeconds (`/Game/Resource_Game_Instance.Flint` _game_instance) _mountain false)
  (`/Game/Resource_Game_Instance.Progress++` _game_instance DeltaSeconds (`/Game/Resource_Game_Instance.Ground_Stone` _game_instance) _mountain false)
  (`/Game/Resource_Game_Instance.Progress++` _game_instance DeltaSeconds (`/Game/Resource_Game_Instance.Evil_Spirit` _game_instance) _mountain false))

(fn `UserConstructionScript`)