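; Cave source actor for a resource game, which drives resource progression through the game instance while it is in the level.
; BeginPlay caches the Resource_Game_Instance, then each Tick calls its Progress function for two chained pairs: Air sourced from Homo, and Homo sourced from Cave.
; The construction script sets the actor to a fixed rotation.
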(event `self.ReceiveBeginPlay`
  ;[1 1 1] BeginPlay
  (bind _asresource_game_instance (cast `/Game/Resource_Game_Instance` (`GameplayStatics.GetGameInstance`)))
  (set `self.Game Instance` _asresource_game_instance))

(event `self.ReceiveTick`
  (params (DeltaSeconds :type "Float (single-precision)"))
  (bind _game_instance (`self.Game Instance`))
  ;[1 1 1] Tick
  (`/Game/Resource_Game_Instance.Progress++` _game_instance DeltaSeconds (`/Game/Resource_Game_Instance.Air` _game_instance) (`/Game/Resource_Game_Instance.Homo` _game_instance))
  (`/Game/Resource_Game_Instance.Progress++` _game_instance DeltaSeconds (`/Game/Resource_Game_Instance.Homo` _game_instance) (`/Game/Resource_Game_Instance.Cave` _game_instance)))

(fn `UserConstructionScript`
  (`self.SetActorRotation` (struct :`Yaw` 100.0)))