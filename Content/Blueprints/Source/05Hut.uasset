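; Hut source Blueprint that drives resource progress for a Hut in the game's resource system.
; On BeginPlay it caches the Resource_Game_Instance.
; Every tick it calls the instance's Progress for Basic Tool, Weapon, Pelt and Wheel with Hut as the source, so progress logic lives in the game instance.
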(event `self.ReceiveBeginPlay`
  (bind _asresource_game_instance (cast `/Game/Resource_Game_Instance` (`GameplayStatics.GetGameInstance`)))
  (set `self.Game Instance` _asresource_game_instance))

(event `self.ReceiveTick`
  (params (DeltaSeconds :type "Float (single-precision)"))
  (bind _game_instance (`self.Game Instance`))
  (bind _hut (`/Game/Resource_Game_Instance.Hut` _game_instance))
  (`/Game/Resource_Game_Instance.Progress++` _game_instance DeltaSeconds (`/Game/Resource_Game_Instance.Basic_Tool` _game_instance) _hut false)
  (`/Game/Resource_Game_Instance.Progress++` _game_instance DeltaSeconds (`/Game/Resource_Game_Instance.Weapon` _game_instance) _hut false)
  (`/Game/Resource_Game_Instance.Progress++` _game_instance DeltaSeconds (`/Game/Resource_Game_Instance.Pelt` _game_instance) _hut false)
  (`/Game/Resource_Game_Instance.Progress++` _game_instance DeltaSeconds (`/Game/Resource_Game_Instance.Wheel` _game_instance) _hut false))

(fn `UserConstructionScript`)