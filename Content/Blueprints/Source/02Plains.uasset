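; Plains source actor that drives resource progression for the Soil, Clay, Sand and EvilSpirit elements.
; BeginPlay caches the Resource_Game_Instance, and Tick calls its Progress function for each element with Plains as the source.
; On every tick where Soil is exactly level 85, it increments Path's count and availability and unlocks Forest and Mountain.
; The construction script sets a fixed actor rotation.
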(event `self.ReceiveBeginPlay`
  ;[1 1 1] BeginPlay
  (bind _asresource_game_instance (cast `/Game/Resource_Game_Instance` (`GameplayStatics.GetGameInstance`)))
  (set `self.Game Instance` _asresource_game_instance))

(event `self.ReceiveTick`
  (params (DeltaSeconds :type "Float (single-precision)"))
  (bind _game_instance (`self.Game Instance`))
  (bind _plains (`/Game/Resource_Game_Instance.Plains` _game_instance))
  (bind _soil (`/Game/Resource_Game_Instance.Soil` _game_instance))
  (bind _path (`/Game/Resource_Game_Instance.Path` (`self.Game Instance`)))
  (bind (_name _locked _count _level _available) (break `/Game/Blueprints/Struct/Element` _path))
  (`/Game/Resource_Game_Instance.Progress++` _game_instance DeltaSeconds _soil _plains)
  (if (== (`.Level_58_CDBECD304FD61C06C6C1108C2EC9D6C3` (break `/Game/Blueprints/Struct/Element` _soil)) 85)
    (setmembers `/Game/Blueprints/Struct/Element` :`StructRef` _path :`Count` (+ _count 1) :`Available` (+ _available 1))
    (setmembers `/Game/Blueprints/Struct/Element` :`StructRef` (`/Game/Resource_Game_Instance.Forest` (`self.Game Instance`)) :`Locked` false)
    (setmembers `/Game/Blueprints/Struct/Element` :`StructRef` (`/Game/Resource_Game_Instance.Mountain` (`self.Game Instance`)) :`Locked` false))
  (`/Game/Resource_Game_Instance.Progress++` _game_instance DeltaSeconds (`/Game/Resource_Game_Instance.Clay` _game_instance) _plains)
  (`/Game/Resource_Game_Instance.Progress++` _game_instance DeltaSeconds (`/Game/Resource_Game_Instance.Sand` _game_instance) _plains)
  (`/Game/Resource_Game_Instance.Progress++` _game_instance DeltaSeconds (`/Game/Resource_Game_Instance.Evil_Spirit` _game_instance) _plains))

(fn `UserConstructionScript`
  (`self.SetActorRotation` (struct :`Yaw` 35.0)))