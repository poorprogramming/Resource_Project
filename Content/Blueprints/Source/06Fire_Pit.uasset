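; Fire Pit resource source Blueprint that drives production of Fire, Potash, Meat and Clay Pot.
; BeginPlay casts and caches the Resource Game Instance.
; Every Tick it calls the game instance's Progress for each of those elements, passing delta time and the FirePit source, so the progression logic itself lives in the game instance.
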(event `self.ReceiveBeginPlay`
  (bind _asresource_game_instance (cast `/Game/Resource_Game_Instance` (`GameplayStatics.GetGameInstance`)))
  (set `self.Game Instance` _asresource_game_instance))

(event `self.ReceiveTick`
  (params (DeltaSeconds :type "Float (single-precision)"))
  (bind _game_instance (`self.Game Instance`))
  (bind _fire_pit (`/Game/Resource_Game_Instance.Fire_Pit` _game_instance))
  (`/Game/Resource_Game_Instance.Progress++` _game_instance DeltaSeconds (`/Game/Resource_Game_Instance.Fire` _game_instance) _fire_pit false)
  (`/Game/Resource_Game_Instance.Progress++` _game_instance DeltaSeconds (`/Game/Resource_Game_Instance.Potash` _game_instance) _fire_pit false)
  (`/Game/Resource_Game_Instance.Progress++` _game_instance DeltaSeconds (`/Game/Resource_Game_Instance.Meat` _game_instance) _fire_pit false)
  (`/Game/Resource_Game_Instance.Progress++` _game_instance DeltaSeconds (`/Game/Resource_Game_Instance.Clay_Pot` _game_instance) _fire_pit false))

(fn `UserConstructionScript`)