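; Altar Blueprint that advances the Medicine, SpokenWord, God and Rain elements held by the game instance.
; BeginPlay casts and caches the Resource_Game_Instance.
; Each Tick calls the instance's Progress once per element, passing delta time and the instance's Altar as the source, so the progression logic itself lives in the game instance.
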(event `self.ReceiveBeginPlay`
  (bind _asresource_game_instance (cast `/Game/Resource_Game_Instance` (`GameplayStatics.GetGameInstance`)))
  (set `self.Game Instance` _asresource_game_instance))

(event `self.ReceiveTick`
  (params (DeltaSeconds :type "Float (single-precision)"))
  (bind _game_instance (`self.Game Instance`))
  (bind _altar (`/Game/Resource_Game_Instance.Altar` _game_instance))
  (`/Game/Resource_Game_Instance.Progress++` _game_instance DeltaSeconds (`/Game/Resource_Game_Instance.Medicine` _game_instance) _altar false)
  (`/Game/Resource_Game_Instance.Progress++` _game_instance DeltaSeconds (`/Game/Resource_Game_Instance.Spoken_Word` _game_instance) _altar false)
  (`/Game/Resource_Game_Instance.Progress++` _game_instance DeltaSeconds (`/Game/Resource_Game_Instance.God` _game_instance) _altar false)
  (`/Game/Resource_Game_Instance.Progress++` _game_instance DeltaSeconds (`/Game/Resource_Game_Instance.Rain` _game_instance) _altar false))

(fn `UserConstructionScript`)