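; Forest resource source actor that drives production of its four resources: softwood, fruit, herbs and wild game.
; On BeginPlay it casts the game instance to Resource_Game_Instance and caches it.
; Every Tick it calls the game instance's Progress once per resource, passing delta time, that element and the Forest source, so the progression logic itself lives in the game instance.
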(event `self.ReceiveBeginPlay`
  (bind _asresource_game_instance (cast `/Game/Resource_Game_Instance` (`GameplayStatics.GetGameInstance`)))
  (set `self.Game Instance` _asresource_game_instance))

(event `self.ReceiveTick`
  (params (DeltaSeconds :type "Float (single-precision)"))
  (bind _game_instance (`self.Game Instance`))
  (bind _forest (`/Game/Resource_Game_Instance.Forest` _game_instance))
  (`/Game/Resource_Game_Instance.Progress++` _game_instance DeltaSeconds (`/Game/Resource_Game_Instance.Softwood` _game_instance) _forest)
  (`/Game/Resource_Game_Instance.Progress++` _game_instance DeltaSeconds (`/Game/Resource_Game_Instance.Fruit` _game_instance) _forest)
  (`/Game/Resource_Game_Instance.Progress++` _game_instance DeltaSeconds (`/Game/Resource_Game_Instance.Herbs` _game_instance) _forest)
  (`/Game/Resource_Game_Instance.Progress++` _game_instance DeltaSeconds (`/Game/Resource_Game_Instance.Wild_Game` _game_instance) _forest))

(fn `UserConstructionScript`)