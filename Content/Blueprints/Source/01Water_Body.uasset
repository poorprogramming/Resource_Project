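; Water body resource source actor that drives production of water-related elements in a resource game.
; On BeginPlay it casts the game instance to Resource_Game_Instance and caches it.
; Every Tick it calls the instance's Progress function for Water, Fish, Salt and SeaMonster, passing delta time and the WaterBody source, so the actual progression logic lives in the game instance.
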(event `self.ReceiveBeginPlay`
  ;[1 1 1] BeginPlay
  (bind _asresource_game_instance (cast `/Game/Resource_Game_Instance` (`GameplayStatics.GetGameInstance`)))
  (set `self.Game Instance` _asresource_game_instance))

(event `self.ReceiveTick`
  (params (DeltaSeconds :type "Float (single-precision)"))
  (bind _game_instance (`self.Game Instance`))
  (bind _water_body (`/Game/Resource_Game_Instance.Water_Body` _game_instance))
  (`/Game/Resource_Game_Instance.Progress++` _game_instance DeltaSeconds (`/Game/Resource_Game_Instance.Water` _game_instance) _water_body)
  (`/Game/Resource_Game_Instance.Progress++` _game_instance DeltaSeconds (`/Game/Resource_Game_Instance.Fish` _game_instance) _water_body)
  (`/Game/Resource_Game_Instance.Progress++` _game_instance DeltaSeconds (`/Game/Resource_Game_Instance.Salt` _game_instance) _water_body)
  (`/Game/Resource_Game_Instance.Progress++` _game_instance DeltaSeconds (`/Game/Resource_Game_Instance.Sea_Monster` _game_instance) _water_body))

(fn `UserConstructionScript`)