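; Path actor that defines six named spline routes: horizontal, vertical, and upper and lower variants of L and R.
; The construction script appends hard-coded local-space points to each spline component, shaping flat curves at zero Z.
; The event graph holds only empty events, so the actor supplies path geometry and has no runtime logic of its own.
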(event `self.ReceiveBeginPlay`)

(event `self.ReceiveActorBeginOverlap`
  (params (OtherActor :type "Actor Object Reference")))

(event `self.ReceiveTick`
  (params (DeltaSeconds :type "Float (single-precision)")))

(fn `UserConstructionScript`
  ;[1 1 1] Path_Splines
  ;;[1 1 1] Horizontal
  (`SplineComponent.AddSplinePoint` (`self.Spline_Horizontal`) (`KismetMathLibrary.MakeVector` 200.0 -4.0) "Local")
  (`SplineComponent.AddSplinePoint` (`self.Spline_Horizontal`) (`KismetMathLibrary.MakeVector` 300.0 -7.0) "Local")
  (`SplineComponent.AddSplinePoint` (`self.Spline_Horizontal`) (`KismetMathLibrary.MakeVector` 400.0 -11.0) "Local")
  ;;[1 1 1] Vertical
  (`SplineComponent.AddSplinePoint` (`self.Spline_Vertical`) (`KismetMathLibrary.MakeVector` 35.0 -32.0) "Local")
  (`SplineComponent.AddSplinePoint` (`self.Spline_Vertical`) (`KismetMathLibrary.MakeVector` 110.0 -74.0) "Local")
  (`SplineComponent.AddSplinePoint` (`self.Spline_Vertical`) (`KismetMathLibrary.MakeVector` 165.0 -68.0) "Local")
  (`SplineComponent.AddSplinePoint` (`self.Spline_Vertical`) (`KismetMathLibrary.MakeVector` 200.0 -82.0) "Local")
  ;;[1 1 1] L_Upper
  (`SplineComponent.AddSplinePoint` (`self.Spline_L_Upper`) (`KismetMathLibrary.MakeVector` 40.0 -32.0) "Local")
  (`SplineComponent.AddSplinePoint` (`self.Spline_L_Upper`) (`KismetMathLibrary.MakeVector` 130.0 -38.0) "Local")
  (`SplineComponent.AddSplinePoint` (`self.Spline_L_Upper`) (`KismetMathLibrary.MakeVector` 260.0 -9.0) "Local")
  ;;[1 1 1] L_Lower
  (`SplineComponent.AddSplinePoint` (`self.Spline_L_Lower`) (`KismetMathLibrary.MakeVector` 120.0 16.0) "Local")
  (`SplineComponent.AddSplinePoint` (`self.Spline_L_Lower`) (`KismetMathLibrary.MakeVector` 300.0 10.0) "Local")
  (`SplineComponent.AddSplinePoint` (`self.Spline_L_Lower`) (`KismetMathLibrary.MakeVector` 360.0 -45.5) "Local")
  ;;[1 1 1] R_Upper
  (`SplineComponent.AddSplinePoint` (`self.Spline_R_Upper`) (`KismetMathLibrary.MakeVector` 38.0 -30.0 0.0) "Local")
  (`SplineComponent.AddSplinePoint` (`self.Spline_R_Upper`) (`KismetMathLibrary.MakeVector` 50.0 -55.0) "Local")
  (`SplineComponent.AddSplinePoint` (`self.Spline_R_Upper`) (`KismetMathLibrary.MakeVector` -40.0 -70.0) "Local")
  ;;[1 1 1] R_Lower
  (`SplineComponent.AddSplinePoint` (`self.Spline_R_Lower`) (`KismetMathLibrary.MakeVector` 108.0 16.0 0.0) "Local")
  (`SplineComponent.AddSplinePoint` (`self.Spline_R_Lower`) (`KismetMathLibrary.MakeVector` 260.0 25.0) "Local")
  (`SplineComponent.AddSplinePoint` (`self.Spline_R_Lower`) (`KismetMathLibrary.MakeVector` 273.0 53.0) "Local"))